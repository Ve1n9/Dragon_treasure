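; Inventory component that stores an array of item objects and toggles the inventory screen.
; On BeginPlay it fills the Inventory array with BP_baseitemobject instances given randomly chosen images, which looks like test content.
; Toggleinventory creates or removes the UI_Inventory_Grid widget, using the stored reference as the open state, and switches mouse cursor and input mode to match.
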(event `self.ReceiveBeginPlay`
  (for _ (range 16)
    (bind _returnvalue (`|GenericCreateObject` self "/Game/Blueprints/inventory/BP_baseitemobject.BP_baseitemobject_C" (select `int` (`KismetMathLibrary.RandomIntegerInRange` 0 2) :`0` "/Game/Levels/6620f6fe27f0d70001f4d6fd.6620f6fe27f0d70001f4d6fd" :`1` "/Game/content/White-Circle-PNG-HD-Image.White-Circle-PNG-HD-Image" :`2` "/Game/StarterContent/Textures/T_Brick_Clay_Beveled_D.T_Brick_Clay_Beveled_D" :!type "Texture2D Object Reference")))
    (`KismetArrayLibrary.Array_Add` (`self.Inventory`) _returnvalue)))

(fn `Toggleinventory`
  (bind _returnvalue (`GameplayStatics.GetPlayerController` 0))
  (bind _returnvalue_2 (`GameplayStatics.GetPlayerController` 0))
  (bind _ui_inventoryreference (`self.UI_InventoryReference`)
    (:`then`
      (`Widget.RemoveFromParent` _ui_inventoryreference)
      (set `PlayerController.bShowMouseCursor` false _returnvalue)
      (`WidgetBlueprintLibrary.SetInputMode_GameOnly` _returnvalue)
      (set `self.UI_InventoryReference` null))
    (:`else`
      (bind _returnvalue_3 (`|CreateWidget` "/Game/Blueprints/widgets/UI_Inventory_Grid.UI_Inventory_Grid_C"))
      (bind _output_get (set `self.UI_InventoryReference` _returnvalue_3))
      (`UserWidget.AddToViewport` _output_get 0)
      (set `PlayerController.bShowMouseCursor` true _returnvalue_2)
      (`WidgetBlueprintLibrary.SetInputMode_GameAndUIEx` _returnvalue_2 (`self.UI_InventoryReference`)))))